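; UpgradeBerry is a one-use interactable actor that opens the upgrade menu when the player presses E near it.
; Its trigger volume enables the actor's input for player controller 0 on begin overlap and disables it on end overlap, without checking which actor overlapped.
; Pressing E creates the UpgradeMenu widget if needed, displays it with UI-only input, pauses the game and destroys the berry.
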(event `self.Trigger Volume.OnComponentBeginOverlap`
  (params (OtherActor :type "Actor Object Reference") (OtherComp :type "PrimitiveComponent Object Reference") (OtherBodyIndex :type Integer) (bFromSweep :type Boolean) (SweepResult :type "HitResult Structure (by ref)"))
  ;[1 1 1] OnTriggerEnter enable player input
  (`self.EnableInput` (`GameplayStatics.GetPlayerController` 0)))

(event `self.Trigger Volume.OnComponentEndOverlap`
  (params (OtherActor :type "Actor Object Reference") (OtherComp :type "PrimitiveComponent Object Reference") (OtherBodyIndex :type Integer))
  ;[1 1 1] OnTriggerExit disable player input
  (`self.DisableInput` (`GameplayStatics.GetPlayerController` 0)))

(event `Key|E`
  (params (Key :type "Key Structure" :default "AnyKey"))
  ;[1 1 1] Show Upgrade Menu when press 'E'
  (:`Pressed`
    (`/Engine/EditorBlueprintResources/StandardMacros.IsValid` (`self.UpgradeMenuReference`)
      (:`Is Valid`
        _)
      (:`Is Not Valid`
        (bind _returnvalue (`|CreateWidget` "/Game/Blueprints/UpgradeMenu.UpgradeMenu_C"))
        (set `self.UpgradeMenuReference` _returnvalue)))
    (`WidgetBlueprintLibrary.SetInputMode_UIOnlyEx` null)
    (`UserWidget.AddToViewport` (`self.UpgradeMenuReference`) 0)
    (`GameplayStatics.SetGamePaused` true)
    (`self.K2_DestroyActor`)))

(event `self.ReceiveBeginPlay`)

(event `self.ReceiveActorBeginOverlap`
  (params (OtherActor :type "Actor Object Reference")))

(event `self.ReceiveTick`
  (params (DeltaSeconds :type "Float (single-precision)")))

(fn `UserConstructionScript`)