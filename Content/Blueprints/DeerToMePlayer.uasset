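; Player Blueprint for a deer game, handling the pause menu and a deer-call effect.
; P or gamepad left trigger opens a cached pause widget; BeginPlay sets game input and initial stamina.
; CalledDeer fires a brief electric beam at ClosestDeer's tail, though its search starts from the first deer and clears, rather than assigns, closer matches.
; Hunter-proximity screen tint and vignette logic is present but disconnected.
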(event `Key|P`
  (params (Key :type "Key Structure" :default "AnyKey"))
  (bind _pause_menu_reference (`self.Pause Menu Reference`))
  ;[1 1 1] Pause Menu
  (:`Pressed`
    (`/Engine/EditorBlueprintResources/StandardMacros.IsValid` (`self.Pause Menu Reference`) :!label _label
      (:`Is Valid`
        _)
      (:`Is Not Valid`
        (bind _returnvalue (`|CreateWidget` "/Game/Blueprints/PauseMenu.PauseMenu_C"))
        (set `self.Pause Menu Reference` _returnvalue)))
    (`WidgetBlueprintLibrary.SetInputMode_UIOnlyEx` (`GameplayStatics.GetPlayerController` null) _pause_menu_reference)
    (`UserWidget.AddToViewport` _pause_menu_reference 0)
    (`GameplayStatics.SetGamePaused` null true)))

(event `Key|Gamepad_LeftTrigger`
  (params (Key :type "Key Structure" :default "AnyKey"))
  ;[1 1 1] Pause Menu
  (:`Pressed`
    (goto _label)))

(event `self.ReceiveTick`
  (params (DeltaSeconds :type "Float (single-precision)")))

(event `self.ReceiveActorBeginOverlap`
  (params (OtherActor :type "Actor Object Reference")))

(event `self.ReceiveBeginPlay`
  (bind _seconds (`GameplayStatics.GetAccurateRealTime` null))
  ;[1 1 1] Set up input
  (`WidgetBlueprintLibrary.SetInputMode_GameOnly` (`GameplayStatics.GetPlayerController` null))
  (set `self.InitialStamina` 1000.0)
  (`KismetMathLibrary.SetRandomStreamSeed` (`KismetMathLibrary.MakeRandomStream` _seconds) _seconds))

(event `self.CalledDeer`
  (bind _outactors (`GameplayStatics.GetAllActorsOfClass` null "/Game/Ai/DeerAIObject.DeerAIObject_C"))
  (for (_array_element _array_index) _outactors
    (if (== _array_index 0)
      (set `self.ClosestDeer` _array_element)
      (else
        (bind _returnvalue (`self.GetDistanceTo` (`GameplayStatics.GetPlayerCharacter` null) _array_element))
        (if (< _returnvalue (`self.ClosestDistance`))
          (set `self.ClosestDeer` null)
          (set `self.ClosestDistance` _returnvalue)))))
  (bind _returnvalue_2 (`GameplayStatics.SpawnEmitterAttached` "/Game/ExampleContent/Effects/ParticleSystems/P_electricity_arc.P_electricity_arc" (`self.CapsuleComponent`) "None" (0.0 0.0 0.0) (struct) "SnapToTargetIncludingScale"))
  (set `self.bPlayParticles` true)
  (`ParticleSystemComponent.SetBeamTargetPoint` _returnvalue_2 0 (`SceneComponent.GetSocketLocation` (`Character.Mesh` (`self.ClosestDeer`)) "RigTail1") 0)
  (`KismetSystemLibrary.Delay` null 3.0)
  (`SceneComponent.DetachFromParent` _returnvalue_2 false true)
  (`ActorComponent.K2_DestroyComponent` _returnvalue_2))

(fn `UserConstructionScript`)